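; BP_GUNTESTINGCHAR is a player character, apparently for testing guns, with basic movement, jump and sensitivity-scaled look controls.
; On BeginPlay it spawns a BP_PistolGun as CurrentGun, passes itself and its Camera to SetupWeapon, and attaches the gun to the character Mesh.
; The Fire input delegates to the gun's own Fire function after a validity check, so the character holds no shooting logic.
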(event EventBeginPlay
  (bind _self self)
  (bind _returnvalue (Game|SpawnActorfromClass "/Game/Player/Blueprint/BP_PistolGun.BP_PistolGun_C" (Math|Transform|MakeTransform "0, 0, 0") "AlwaysSpawn" _self _self))
  (bind _output_get (Variables|Default|SetCurrentGun _returnvalue))
  (Class|BaseGun|SetupWeapon _output_get self (Variables|Default|GetCamera))
  (Transformation|AttachComponentToComponent _output_get (Variables|Character|GetMesh) "None" "SnapToTarget" "KeepRelative" "KeepRelative" true))

(event EventTick
  (params (DeltaSeconds :type Float%20%28single-precision%29)))

(event Input|ActionEvents|InputActionJump
  (params (Key :type Key%20Structure :default "None"))
  (:Pressed
    (Character|Jump)))

(event Input|ActionEvents|InputActionFire
  (params (Key :type Key%20Structure :default "None"))
  (bind _currentgun (Variables|Default|GetCurrentGun))
  (:Pressed
    (Utilities|IsValid _currentgun
      (:Is%20Valid
        (Class|SingleFireGun|Fire _currentgun)))))

(event Input|AxisEvents|InputAxisMoveForward
  (params (AxisValue :type Float%20%28single-precision%29))
  (Pawn|Input|AddMovementInput (Math|Vector|GetForwardVector (Transformation|GetActorRotation)) AxisValue false))

(event Input|AxisEvents|InputAxisMoveRight
  (params (AxisValue :type Float%20%28single-precision%29))
  (Pawn|Input|AddMovementInput (Math|Vector|GetRightVector (Transformation|GetActorRotation)) AxisValue false))

(event Input|AxisEvents|InputAxisLookUp
  (params (AxisValue :type Float%20%28single-precision%29))
  (Pawn|Input|AddControllerPitchInput (* (Variables|Default|Getsensitivity) AxisValue)))

(event Input|AxisEvents|InputAxisTurn
  (params (AxisValue :type Float%20%28single-precision%29))
  (Pawn|Input|AddControllerYawInput (* AxisValue (Variables|Default|Getsensitivity))))

(fn ConstructionScript)