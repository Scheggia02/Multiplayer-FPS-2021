(event EventBeginPlay
  (Variables|Default|SetHealth (Variables|Default|GetMaxHealth))
  (Variables|Default|SetisDead false))

(fn ApplyDamage
  (params (Damage :type Float%20%28single-precision%29))
  (if (not (Variables|Default|GetisDead))
    (bind _output_get (Variables|Default|SetHealth (Math|Float|Clamp(Float) (- (Variables|Default|GetHealth) Damage) 0.0 (Variables|Default|GetMaxHealth))))
    (if (== _output_get 0.0)
      (Variables|Default|SetisDead true)
      (CallFunction|OnDeath))))

(fn ApplyCure
  (params (Cure :type Float%20%28single-precision%29))
  (if (not (Variables|Default|GetisDead))
    (if (< (Variables|Default|GetHealth) (Variables|Default|GetMaxHealth))
      (Variables|Default|SetHealth (+ (Variables|Default|GetHealth) Cure)))))

(fn OnDeath
  (Development|PrintString "SEI MORTO"))