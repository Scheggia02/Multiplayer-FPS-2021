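; Player character Blueprint that handles movement, look, jump and hold-to-crouch input.
; Movement axes follow actor rotation and are gated by CanMove, while look input is scaled by Sensitivity.
; Custom crouch switches MovementMode, applies speed and jump velocity from the MovementModesInfo map, and resizes the capsule and moves the spring arm directly, without a headroom check on release.
; Tick prints the current speed on screen for debugging.
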(event EventTick
  (params (DeltaSeconds :type Float%20%28single-precision%29))
  (Development|PrintString (Utilities|String|ToString(Float) (Math|Vector|VectorLength (Transformation|GetVelocity))) true true "(R=0.000000,G=0.660000,B=1.000000,A=1.000000)" DeltaSeconds))

(event Input|ActionEvents|InputActionJump
  (params (Key :type Key%20Structure :default "None"))
  (:Pressed
    (Character|Jump)))

(event Input|ActionEvents|InputActionCrouch
  (params (Key :type Key%20Structure :default "None"))
  (:Pressed
    (CallFunction|StartCrouching))
  (:Released
    (CallFunction|StopCrouching)))

(event Input|AxisEvents|InputAxisMoveForward
  (params (AxisValue :type Float%20%28single-precision%29))
  (if (Variables|Default|GetcanMove)
    (Pawn|Input|AddMovementInput (Math|Vector|GetForwardVector (Transformation|GetActorRotation)) AxisValue false)))

(event Input|AxisEvents|InputAxisMoveRight
  (params (AxisValue :type Float%20%28single-precision%29))
  (if (Variables|Default|GetcanMove)
    (Pawn|Input|AddMovementInput (Math|Vector|GetRightVector (Transformation|GetActorRotation)) AxisValue false)))

(event Input|AxisEvents|InputAxisLookUp
  (params (AxisValue :type Float%20%28single-precision%29))
  (Pawn|Input|AddControllerPitchInput (* (Variables|Default|Getsensitivity) AxisValue)))

(event Input|AxisEvents|InputAxisTurn
  (params (AxisValue :type Float%20%28single-precision%29))
  (Pawn|Input|AddControllerYawInput (* AxisValue (Variables|Default|Getsensitivity))))

(fn ConstructionScript)

(fn StartCrouching
  (bind _movementmodesinfo (Variables|Default|GetMovementModesInfo))
  (bind _charactermovement (Variables|Character|GetCharacterMovement))
  (bind _value (Utilities|Map|Find _movementmodesinfo "NewEnumerator1"))
  (Variables|Default|SetmovementMode "NewEnumerator1")
  (Variables|/Script/Engine.CharacterMovementComponent|SetMaxWalkSpeed _charactermovement (.movementspeed _value))
  (Variables|/Script/Engine.CharacterMovementComponent|SetJumpZVelocity _charactermovement (.jumpvelocity _value))
  (Transformation|SetRelativeLocation (Variables|Default|GetSpringArm) "0, 0,10.000000" false false)
  (Components|Capsule|SetCapsuleHalfHeight (Variables|Collision|GetCapsuleComponent) 44.0 true))

(fn StopCrouching
  (bind _movementmodesinfo (Variables|Default|GetMovementModesInfo))
  (bind _charactermovement (Variables|Character|GetCharacterMovement))
  (bind _value (Utilities|Map|Find _movementmodesinfo "NewEnumerator0"))
  (Variables|Default|SetmovementMode "NewEnumerator0")
  (Variables|/Script/Engine.CharacterMovementComponent|SetMaxWalkSpeed _charactermovement (.movementspeed _value))
  (Variables|/Script/Engine.CharacterMovementComponent|SetJumpZVelocity _charactermovement (.jumpvelocity _value))
  (Transformation|SetRelativeLocation (Variables|Default|GetSpringArm) "0, 0,50.000000" false false)
  (Components|Capsule|SetCapsuleHalfHeight (Variables|Collision|GetCapsuleComponent) 88.0 true))